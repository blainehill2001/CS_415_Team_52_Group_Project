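; Hurricane enemy character for a rock-paper-scissors game, setting its own sprite and form on spawn.
; Each tick it moves along the Attack vector, or wanders in a random direction when the player is high up or in form 3.
; Player contact uses Compare to do nothing, print game over or bounce; enemy contact bounces, re-rolling the wander direction.
; The RunAway steering and discrete direction picker are disconnected.
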(event EventBeginPlay
  (CallFunction|UpdateSprite 3)
  (Variables|Default|SetForm "NewEnumerator3")
  (Variables|Default|Setdir (Math|Vector|MakeVector (Math|Random|RandomFloatinRange -1.0 1.0) (Math|Random|RandomFloatinRange -1.0 1.0) 0.0))
  (Variables|Default|SetAttackPlayer (Math|Random|RandomBoolwithWeight 1.0)))

(event Collision|EventActorBeginOverlap
  (params (OtherActor :type Actor%20Object%20Reference))
  (|CallParentFunction OtherActor))

(event EventHandleEnemyEnemyInteraction
  (params (enemy1 :type BP%20RPS%20Enemy%20Object%20Reference) (enemy2 :type BP%20RPS%20Enemy%20Object%20Reference))
  (CallFunction|Bounce enemy1))

(event EventHandlePlayerEnemyInteraction
  (params (player :type BP%20RPS%20Player%20Object%20Reference) (enemy :type BP%20RPS%20Enemy%20Object%20Reference))
  (bind _win (CallFunction|Compare player enemy))
  (if (not (== _win 2))
    (if (== _win 0)
      (Development|PrintString "game over (from enemy's perspective)" false)
      (else
        (CallFunction|Bounce enemy)))))

(event EventTick
  (params (DeltaSeconds :type Float%20%28single-precision%29))
  (bind _returnvalue (Game|Player|GetPlayerPawn 0))
  (bind _returnvalue_2 (Math|Random|RandomFloatinRange 0.4 1.0))
  (bind _returnvalue_3 (Transformation|GetActorLocation _returnvalue))
  (bind _asbp_rps_player (Utilities|Casting|CastToBP_RPS_Player _returnvalue))
  (if (> (.Z (Math|Vector|BreakVector _returnvalue_3)) 247.0)
    (Variables|Default|SetRunaway true)
    (else
      (Variables|Default|SetRunaway false)
      (if (== (Variables|/Game/RockPaperScissors/BP_RPS_Parent.BP_RPS_Parent_C|GetForm _asbp_rps_player) 3)
        (Variables|Default|SetRunaway true)
        (else
          (Variables|Default|SetRunaway false)))))
  (if (Variables|Default|GetRunaway)
    (if (< (Math|Vector|Distance(Vector) (Transformation|GetActorLocation) _returnvalue_3) 4e+02)
      _
      (else
        _))
    (Pawn|Input|AddMovementInput (Variables|Default|Getdir) _returnvalue_2 false :!label _label)
    (elif (Variables|Default|GetAttackPlayer)
      (bind _position (CallFunction|Attack))
      (Pawn|Input|AddMovementInput _position _returnvalue_2 false)
      (else
        (goto _label)))))

(fn ConstructionScript
  (|CallParentFunction))

(fn NewFunction0)

(fn Bounce
  (Variables|Default|Setdir (Math|Vector|MakeVector (Math|Random|RandomFloatinRange -1.0 1.0) (Math|Random|RandomFloatinRange -1.0 1.0) 0.0)))