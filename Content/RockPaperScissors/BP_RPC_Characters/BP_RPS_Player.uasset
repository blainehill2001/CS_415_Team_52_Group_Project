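; BP_RPS_Player is the player character in a rock-paper-scissors game, resolving encounters with enemies and tracking score and rounds.
; On player-enemy interaction, Compare decides the outcome: a win destroys the enemy, adds score and decrements the Enemy_Spawner's count.
; A loss deducts score, then either uses up a round and teleports the player to a hard-coded location or restarts the level when none remain.
; It also plays music on BeginPlay.
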(event EventBeginPlay
  (|CallParentFunction)
  (Audio|PlaySound2D "/Game/RockPaperScissors/Gundam_Thunderbolt_OST_01_-_Thunderbolt_For_Main_Theme__Io_Fleming_Song_.Gundam_Thunderbolt_OST_01_-_Thunderbolt_For_Main_Theme__Io_Fleming_Song_" 1.0 1.0 0.0 0 0))

(event Collision|EventActorBeginOverlap
  (params (OtherActor :type Actor%20Object%20Reference))
  (|CallParentFunction OtherActor) ; This node is disabled and will not be called.\nDrag off pins to build functionality.
)

(event EventTick
  (params (DeltaSeconds :type Float%20%28single-precision%29))
  (|CallParentFunction DeltaSeconds))

(event EventHandleEnemyEnemyInteraction
  (params (enemy1 :type BP%20RPS%20Enemy%20Object%20Reference) (enemy2 :type BP%20RPS%20Enemy%20Object%20Reference)))

(event EventHandlePlayerEnemyInteraction
  (params (player :type BP%20RPS%20Player%20Object%20Reference) (enemy :type BP%20RPS%20Enemy%20Object%20Reference))
  (bind _win (Default|Compare player player enemy))
  (if (== _win 2)
    (Actor|DestroyActor enemy)
    (Variables|Default|SetScore (+ 1e+01 (Variables|Default|GetScore)))
    (Development|PrintString (Utilities|String|ToString(Float) (Variables|Default|GetScore)))
    (bind _returnvalue (Actor|GetActorOfClass "/Game/RockPaperScissors/Enemy_Spawner.Enemy_Spawner_C"))
    (Variables|/Game/RockPaperScissors/Enemy_Spawner.Enemy_Spawner_C|SetNumber%20of%20Enemies _returnvalue (- (Variables|/Game/RockPaperScissors/Enemy_Spawner.Enemy_Spawner_C|GetNumber%20of%20Enemies _returnvalue) 1))
    (elif (== _win 0)
      (Variables|Default|SetScore (- (Variables|Default|GetScore) 1e+01))
      (Development|PrintString (Utilities|String|ToString(Float) (Variables|Default|GetScore)))
      (Development|PrintString (Utilities|String|ToString(Float) (Variables|Default|GetRoundsLeft)) true true "(R=1.000000,G=0.227347,B=0.313753,A=1.000000)")
      (if (== (Variables|Default|GetRoundsLeft) 0.0)
        (Development|PrintString "game over (from player's perspective)")
        (CallFunction|GameOver)
        (else
          (Variables|Default|SetRoundsLeft (- (Variables|Default|GetRoundsLeft) 1.0))
          (Development|PrintString "move player to PlayerStart and respawn enemies")
          (CallFunction|RespawnPlayer))))))

(fn ConstructionScript
  (|CallParentFunction))

(fn GameOver
  (bind _returnvalue (Game|GetPlayerController 0))
  (Input|SetInputModeGameOnly _returnvalue false)
  (Variables|/Script/Engine.PlayerController|SetbShowMouseCursor _returnvalue false)
  (Development|ExecuteConsoleCommand "restartlevel" 0))

(fn RespawnPlayer
  (Transformation|Teleport "1442.262964,1904.374585,332.011305" "0, 0, 0"))